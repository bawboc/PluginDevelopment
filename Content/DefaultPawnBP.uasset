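; Default pawn Blueprint that serves as a debug driver for quest progression.
; Number keys 1 through 5 each call UpdateQuests on a QuestStatus reference with a different quest event, such as killing the dragon, knight state changes or talking to NPCs.
; BeginPlay, overlap, Tick and the construction script hold no logic.
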(event `Key|One`
  (params (Key :type "Key Structure"))
  (:`Pressed`
    (`QuestStatus.UpdateQuests` (`self.QuestStatus`) "/Game/Quests/InputAtom/KillDragon.KillDragon")))

(event `Key|Two`
  (params (Key :type "Key Structure"))
  (:`Pressed`
    (`QuestStatus.UpdateQuests` (`self.QuestStatus`) "/Game/Quests/InputAtom/KnightBecomesHostile.KnightBecomesHostile")))

(event `Key|Three`
  (params (Key :type "Key Structure"))
  (:`Pressed`
    (`QuestStatus.UpdateQuests` (`self.QuestStatus`) "/Game/Quests/InputAtom/KnightDies.KnightDies")))

(event `Key|Four`
  (params (Key :type "Key Structure"))
  (:`Pressed`
    (`QuestStatus.UpdateQuests` (`self.QuestStatus`) "/Game/Quests/InputAtom/TalkToKnight.TalkToKnight")))

(event `Key|Five`
  (params (Key :type "Key Structure"))
  (:`Pressed`
    (`QuestStatus.UpdateQuests` (`self.QuestStatus`) "/Game/Quests/InputAtom/TalkToWizard.TalkToWizard")))

(fn `UserConstructionScript`)